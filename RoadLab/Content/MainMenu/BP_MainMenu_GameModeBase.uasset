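; Main menu game mode that launches road graph processing for a location given by latitude, longitude and diameter.
; EnterButtonPressed stores the three inputs, lazily constructs a RoadGraphEngineAcess object if none is valid, then calls its StartProcess with them.
; BeginPlay, Tick and the construction script are empty, and a debug print of the inputs is left disconnected.
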(event EventBeginPlay)

(event EventTick
  (params (DeltaSeconds :type Float%20%28single-precision%29)))

(fn ConstructionScript)

(fn EnterButtonPressed
  (params (lat :type Float%20%28double-precision%29) (lon :type Float%20%28double-precision%29) (diam :type Float%20%28double-precision%29))
  (LocalVariables|SetLat_var lat)
  (LocalVariables|SetLon_var lon)
  (LocalVariables|SetDiam_var diam)
  (if (Utilities|IsValid (Variables|Default|GetRoadGraph))
    _
    (else
      (bind _returnvalue (Game|ConstructObjectfromClass "/Script/RoadLab.RoadGraphEngineAcess"))
      (bind _output_get (Variables|Default|SetRoadGraph _returnvalue))))
  (Class|RoadGraphEngineAcess|StartProcess _output_get (LocalVariables|GetLat_var) (LocalVariables|GetLon_var) (LocalVariables|GetDiam_var)))